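; BP_DoorTwoWays is an interactable door that swings open to either side depending on where the player stands.
; On opening, a dot product of the direction to the player and the actor's forward vector selects the target yaw.
; A timeline interpolates the door's yaw from closed to that angle.
; A FlipFlop alternates between opening and reversing the timeline, and interactions during playback are ignored.
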(event EventOnInteract
  (params (Actor :type Actor%20Object%20Reference) (Player%20Location :type Vector :default "0, 0, 0"))
  (if (not (Audio|Components|Audio|IsPlaying (Variables|Default|GetDoorTimeline)))
    (Utilities|FlowControl|FlipFlop
      (:A
        (CallFunction|SetDoorOpenAngle Player%20Location)
        (bind _door_alpha (Timeline|DoorTimeline Play)
          (:Update
            (Transformation|SetRelativeRotation (Variables|Default|GetDoor) (Math|Rotator|MakeRotator 0.0 0.0 (Math|Float|Lerp 1.8e+02 (Variables|Default|GetDoorOpenAngle) _door_alpha)) false false))))
      (:B
        (Timeline|DoorTimeline Reverse)))))

(fn ConstructionScript)

(fn SetDoorOpenAngle
  (params (Player%20Location :type Vector))
  (Variables|Default|SetDoorOpenAngle (Math|Float|SelectFloat 9e+01 2.7e+02 (>= (Math|Vector|DotProduct (Math|Vector|GetUnitDirection(Vector) (Transformation|GetActorLocation) Player%20Location) (Transformation|GetActorForwardVector)) 0.0)))
  (return))