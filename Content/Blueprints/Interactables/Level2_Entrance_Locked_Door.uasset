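; Interactable Level 2 entrance door that gates passage behind a countdown and triggers a falling-floor sequence.
; An overlap box spawns the countdown widget; interacting while Timer is nonzero teleports the player, otherwise a timeline swings the door open.
; Leaving the Exit volume locks and closes the door, then delayed steps drop the floor and chair, restore them, teleport the player, and swap static doors for normal doors hidden at BeginPlay.
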(event OnComponentBeginOverlap(Box_0)
  (params (OverlappedComponent :type Primitive%20Component%20Object%20Reference) (OtherActor :type Actor%20Object%20Reference) (OtherComp :type Primitive%20Component%20Object%20Reference) (OtherBodyIndex :type Integer) (bFromSweep :type Boolean) (SweepResult :type Hit%20Result%20Structure%20%28by%20ref%29))
  (Utilities|Casting|CastToBP_ThirdPersonCharacter OtherActor)
  (Development|PrintString "Triggered")
  (bind _returnvalue (UserInterface|CreateWidget "/Game/UI/CountdownTimer.CountdownTimer_C"))
  (Variables|Default|SetTimer (Variables|/Game/UI/CountdownTimer.CountdownTimer_C|GetCountdown _returnvalue))
  (UserInterface|Viewport|AddtoViewport _returnvalue 0)
  (Components|DestroyComponent (Variables|Default|GetBox_0))
  (Utilities|FlowControl|Delay 7.0)
  (Variables|Default|SetTimer 0.0))

(event OnComponentEndOverlap(Exit)
  (params (OverlappedComponent :type Primitive%20Component%20Object%20Reference) (OtherActor :type Actor%20Object%20Reference) (OtherComp :type Primitive%20Component%20Object%20Reference) (OtherBodyIndex :type Integer))
  (bind _floor (Variables|Default|GetFloor))
  (bind _floor02 (Variables|Default|GetFloor02))
  (bind _floor_2 (Variables|Default|GetFloor))
  (bind _floor02_2 (Variables|Default|GetFloor02))
  (Utilities|FlowControl|Sequence
    (:then_0
      (Variables|Default|SetCantOpen true)
      (Components|DestroyComponent (Variables|Default|GetExit))
      (bind _door_alpha (Timeline|Timeline_1 Reverse)
        (:Update
          (Transformation|SetRelativeRotation (Variables|Default|GetDoor) (Math|Rotator|MakeRotator 0.0 0.0 (Math|Float|Lerp 1.8e+02 (Variables|Default|GetDoorOpenAngle) _door_alpha)) false false))))
    (:then_1
      (Utilities|FlowControl|Delay 3.0)
      (Rendering|SetActorHiddenInGame _floor_2 true)
      (Collision|SetActorEnableCollision _floor_2 false)
      (Rendering|SetActorHiddenInGame _floor02_2 true)
      (Collision|SetActorEnableCollision _floor02_2 false)
      (Physics|SetSimulatePhysics (Variables|Default|GetFallingFloor) true)
      (Physics|SetSimulatePhysics (Variables|Default|GetChair) true)
      (Utilities|FlowControl|Delay 5.0)
      (Rendering|SetActorHiddenInGame _floor false)
      (Collision|SetActorEnableCollision _floor true)
      (Rendering|SetActorHiddenInGame _floor02 false)
      (Collision|SetActorEnableCollision _floor02 true)
      (bind _asbp_third_person_character (Utilities|Casting|CastToBP_ThirdPersonCharacter (stale EventOnInteract Actor)))
      (Transformation|SetWorldLocation (Variables|/Script/Engine.Character|GetCapsuleComponent _asbp_third_person_character) "430.000000,550.000000,20.000000" false false)
      (Physics|SetSimulatePhysics (Variables|Default|GetChair) false)
      (Transformation|SetWorldTransform (Variables|Default|GetChair) (Math|Transform|MakeTransform "425.000000,100.000000,0.000000" "0, 0, 0" "0.700000,0.700000,0.700000") false false)
      (for _array_element (Variables|Default|GetNormalDoors)
        (Rendering|SetActorHiddenInGame _array_element false)
        (Collision|SetActorEnableCollision _array_element true)
        (for _array_element_2 (Variables|Default|GetStaticDoors)
          (Rendering|SetActorHiddenInGame _array_element_2 true)
          (Collision|SetActorEnableCollision _array_element_2 false))))))

(event EventBeginPlay
  (bind _doortonextlevel (Variables|Default|GetDoorToNextLevel))
  (for _array_element (Variables|Default|GetNormalDoors)
    (Rendering|SetActorHiddenInGame _array_element true)
    (Collision|SetActorEnableCollision _array_element false)
    (Rendering|SetActorHiddenInGame _doortonextlevel true)
    (Collision|SetActorEnableCollision _doortonextlevel false)))

(event EventOnInteract
  (params (Actor :type Actor%20Object%20Reference) (Player%20Location :type Vector :default "0, 0, 0"))
  (if (not (Variables|Default|GetCantOpen))
    (if (== (Variables|Default|GetTimer) 0.0)
      (bind _door_alpha (Timeline|Timeline_1 Play)
        (:Update
          (Transformation|SetRelativeRotation (Variables|Default|GetDoor) (Math|Rotator|MakeRotator 0.0 0.0 (Math|Float|Lerp 1.8e+02 (Variables|Default|GetDoorOpenAngle) _door_alpha)) false false)))
      (else
        (bind _asbp_third_person_character (Utilities|Casting|CastToBP_ThirdPersonCharacter Actor))
        (Transformation|SetWorldLocation (Variables|/Script/Engine.Character|GetCapsuleComponent _asbp_third_person_character) "425.000000,1200.000000,20.000000" false false)))))

(fn ConstructionScript
  (|CallParentFunction))