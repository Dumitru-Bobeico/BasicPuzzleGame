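; BP_Clock is a clock actor in the ClockPuzzle folder that displays the current system time on its hour, minute and second hands.
; From BeginPlay it converts Now() into negative pitch angles and sets each hand's relative rotation, with the hour hand also advancing by the minute.
; A one-second Delay wired back to the start repeats the update indefinitely, so no Tick event is used.
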(event EventBeginPlay
  (bind _returnvalue (Math|DateTime|Now))
  (bind (_year _month _day _hour _minute _second) (Math|DateTime|BreakDateTime _returnvalue))
  (Transformation|SetRelativeRotation (Variables|Default|GetHours) (Math|Rotator|MakeRotator 0.0 (* (+ (* _hour 3e+01) (/ _minute 2.0)) -1.0) 0.0) false false :!label _label)
  (Transformation|SetRelativeRotation (Variables|Default|GetMinutes) (Math|Rotator|MakeRotator 0.0 (* _minute -6.0) 0.0) false false)
  (Transformation|SetRelativeRotation (Variables|Default|GetSeconds) (Math|Rotator|MakeRotator 0.0 (* _second -6.0) 0.0) false false)
  (Utilities|FlowControl|Delay 1.0)
  (goto _label))

(fn ConstructionScript)