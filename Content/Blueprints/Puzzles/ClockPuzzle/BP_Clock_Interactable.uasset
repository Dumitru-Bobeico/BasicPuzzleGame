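; Interactable clock puzzle whose hour, minute and second hands show the current time until the player interacts with it.
; A one-second Delay loop on BeginPlay rotates the hands from Now() and exits once CanChangeClock is set.
; OnInteract sets that flag and starts a looping timer that checks each hand against zero rotation within a tolerance.
; Checks are nested hour, minute, then second, setting solved flags and printing debug strings.
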(event Custom|Check
  (bind _hours (Variables|Default|GetHours))
  (bind _minutes (Variables|Default|GetMinutes))
  (bind _seconds (Variables|Default|GetSeconds))
  (bind _relativerotation (Variables|/Script/Engine.SceneComponent|GetRelativeRotation _seconds))
  (bind _relativerotation_2 (Variables|/Script/Engine.SceneComponent|GetRelativeRotation _hours))
  (bind _relativerotation_3 (Variables|/Script/Engine.SceneComponent|GetRelativeRotation _minutes))
  (Development|PrintString (Utilities|String|ToString(Rotator) _relativerotation_2))
  (if (Utilities|Operators|EqualEqual _relativerotation_2 (Math|Rotator|MakeRotator 0.0 0.0 0.0) (Variables|Default|GetErrorTolerance))
    (Development|PrintString "Clock Hour Puzzle Solved")
    (Variables|Default|SetClockHourSolved true)
    (Development|PrintString (Utilities|String|ToString(Rotator) _relativerotation_3))
    (if (Utilities|Operators|EqualEqual _relativerotation_3 (Math|Rotator|MakeRotator 0.0 0.0 0.0) (Variables|Default|GetErrorTolerance))
      (Development|PrintString "Clock Minute Puzzle Solved")
      (Variables|Default|SetClockMinuteSolved true)
      (Development|PrintString (Utilities|String|ToString(Rotator) _relativerotation))
      (if (Utilities|Operators|EqualEqual _relativerotation (Math|Rotator|MakeRotator 0.0 0.0 0.0) (Variables|Default|GetErrorTolerance))
        (Development|PrintString "Clock Second Puzzle Solved")
        (Variables|Default|SetClockSecondSolved true)))))

(event EventBeginPlay
  (bind _returnvalue (Math|DateTime|Now))
  (bind (_year _month _day _hour _minute _second) (Math|DateTime|BreakDateTime _returnvalue))
  (Transformation|SetRelativeRotation (Variables|Default|GetHours) (Math|Rotator|MakeRotator 0.0 (* _hour -3e+01) 0.0) false false :!label _label)
  (Transformation|SetRelativeRotation (Variables|Default|GetMinutes) (Math|Rotator|MakeRotator 0.0 (* _minute -6.0) 0.0) false false)
  (Transformation|SetRelativeRotation (Variables|Default|GetSeconds) (Math|Rotator|MakeRotator 0.0 (* _second -6.0) 0.0) false false)
  (Utilities|FlowControl|Delay 1.0)
  (if (not (Variables|Default|GetCanChangeClock))
    (goto _label)))

(event EventOnInteract
  (params (Actor :type Actor%20Object%20Reference) (Player%20Location :type Vector :default "0, 0, 0"))
  (Variables|Default|SetCanChangeClock true)
  (Utilities|Time|SetTimerbyEvent (delegate Custom|Check) 0.5 true))

(fn ConstructionScript)