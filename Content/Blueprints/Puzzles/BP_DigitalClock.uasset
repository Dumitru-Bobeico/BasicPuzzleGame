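; BP_DigitalClock is a puzzle-folder Blueprint that displays the current real-world time as a digital clock.
; Every Tick it reads Now, splits it into hour, minute and second, and writes each as integer text to its own text component.
; The construction script is empty, and the file contains no puzzle logic.
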(event EventTick
  (params (DeltaSeconds :type Float%20%28single-precision%29))
  (bind _returnvalue (Math|DateTime|Now))
  (Rendering|Components|TextRender|SetText (Variables|Default|GetCHour) (Utilities|Text|ToText(Integer) (Class|KismetMathLibrary|GetHour _returnvalue)))
  (Rendering|Components|TextRender|SetText (Variables|Default|GetCMinute) (Utilities|Text|ToText(Integer) (Class|KismetMathLibrary|GetMinute _returnvalue)))
  (Rendering|Components|TextRender|SetText (Variables|Default|GetCSecond) (Utilities|Text|ToText(Integer) (Class|KismetMathLibrary|GetSecond _returnvalue))))

(fn ConstructionScript)