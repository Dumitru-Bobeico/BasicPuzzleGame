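; Lap counter for the truck laps puzzle, tracking passes through four numbered checkpoint colliders.
; On BeginPlay it binds LapPuzzle to the exit-collision event of every LapCollider in the level, and each ID sets its own hit flag.
; Exiting collider 4 with 1 to 3 already hit, in any order, increments Laps, prints it and clears the flags.
; No lap target or completion event is present.
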(event Custom|LapPuzzle
  (params (ID :type Integer))
  (if (== ID 1)
    (Variables|Default|SetHit1 true)
    (elif (== ID 2)
      (Variables|Default|SetHit2 true)
      (elif (== ID 3)
        (Variables|Default|SetHit3 true)
        (elif (== ID 4)
          (Variables|Default|SetHit4 true)
          (if (Variables|Default|GetHit1)
            (if (Variables|Default|GetHit2)
              (if (Variables|Default|GetHit3)
                (bind _output_get (Variables|Default|SetLaps (Variables|Default|GetLaps)))
                (Math|Integer|IncrementInt _output_get
                  (:%20%20
                    (Development|PrintString (Utilities|String|ToString(Integer) (Variables|Default|GetLaps)))
                    (Variables|Default|SetHit1 false)
                    (Variables|Default|SetHit2 false)
                    (Variables|Default|SetHit3 false)
                    (Variables|Default|SetHit4 false)))))))))))

(event EventBeginPlay
  (bind _outactors (Actor|GetAllActorsOfClass "/Game/Blueprints/Puzzles/TruckLapsPuzzle/LapCollider.LapCollider_C"))
  (for _array_element _outactors
    (EventDispatchers|BindEventtoOnExitCollision _array_element (delegate Custom|LapPuzzle))))

(fn ConstructionScript)