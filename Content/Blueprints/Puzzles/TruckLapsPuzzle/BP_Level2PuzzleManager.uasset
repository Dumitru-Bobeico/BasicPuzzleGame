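; Manager Blueprint for the Level 2 truck laps puzzle that sets the initial state of five number actors.
; On BeginPlay it calls HideAllNumbers, which hides the actors referenced as One through Five and disables their collision.
; The file contains no logic for revealing the numbers or tracking laps.
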(event EventBeginPlay
  (CallFunction|HideAllNumbers))

(fn ConstructionScript)

(fn HideAllNumbers
  (bind _one (Variables|Default|GetOne))
  (bind _two (Variables|Default|GetTwo))
  (bind _three (Variables|Default|GetThree))
  (bind _four (Variables|Default|GetFour))
  (bind _five (Variables|Default|GetFive))
  (Rendering|SetActorHiddenInGame _one true)
  (Collision|SetActorEnableCollision _one false)
  (Rendering|SetActorHiddenInGame _two true)
  (Collision|SetActorEnableCollision _two false)
  (Rendering|SetActorHiddenInGame _three true)
  (Collision|SetActorEnableCollision _three false)
  (Rendering|SetActorHiddenInGame _four true)
  (Collision|SetActorEnableCollision _four false)
  (Rendering|SetActorHiddenInGame _five true)
  (Collision|SetActorEnableCollision _five false))