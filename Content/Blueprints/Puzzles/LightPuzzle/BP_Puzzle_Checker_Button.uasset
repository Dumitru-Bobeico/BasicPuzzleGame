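; BP_Puzzle_Checker_Button is an interactable button that checks the answer to a colored-light puzzle.
; On interact, it compares each puzzle piece's ColorIndex with the matching ColorCode entry, stopping at the first mismatch.
; A correct code triggers DoorToOpen once through BPI_Interact.
; A wrong code resets every piece to color index zero and refreshes its light.
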(event EventOnInteract
  (params (Actor :type Actor%20Object%20Reference) (Player%20Location :type Vector :default "0, 0, 0"))
  (Variables|Default|SetisCorrect? true)
  (bind (_array_element _array_index) (Utilities|Array|ForEachLoopwithBreak (Variables|Default|GetPuzzlePieces) :!label _label)
    (:LoopBody
      (if (!= (Variables|/Game/Blueprints/Puzzles/LightPuzzle/BP_Light_Puzzle_Piece.BP_Light_Puzzle_Piece_C|GetColorIndex _array_element) (Utilities|Array|Get(acopy) (Variables|Default|GetColorCode) _array_index))
        (Variables|Default|SetisCorrect? false)
        (goto _label Break)))
    (:Completed
      (if (Variables|Default|GetisCorrect?)
        (Utilities|FlowControl|DoOnce false
          (:Completed
            (bind _doortoopen (Variables|Default|GetDoorToOpen)
              (:then
                (if (Utilities|DoesObjectImplementInterface _doortoopen "/Game/Blueprints/Interactables/BPI_Interact.BPI_Interact_C")
                  (Class|BPIInteract|OnInteract(Message) _doortoopen self "0, 0, 0")))
              (:else))))
        (else
          (for _array_element_2 (Variables|Default|GetPuzzlePieces)
            (Variables|/Game/Blueprints/Puzzles/LightPuzzle/BP_Light_Puzzle_Piece.BP_Light_Puzzle_Piece_C|SetColorIndex _array_element_2 0)
            (Default|UpdateLightColor _array_element_2)))))))

(fn ConstructionScript)