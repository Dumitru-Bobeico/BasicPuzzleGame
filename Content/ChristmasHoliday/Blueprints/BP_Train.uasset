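; BP_Train is a holiday train actor that circles a spline-defined track with motor and horn sounds.
; The construction script builds track spline meshes between spline points, with optional loop closure, and places the train mesh at the start.
; A looping timer advances the train's distance by Speed, wrapping at spline length, and updates its location and rotation.
; A motor sound starts on BeginPlay, while a random Delay on Tick spaces horn blasts.
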(event Custom|MoveTrain
  (bind _train (Variables|Default|GetTrain))
  (bind _spline (Variables|Default|GetSpline))
  ;[1 1 1] Move along spline
  (Variables|Default|SetDistance (Math|Float|%(Float) (+ (Variables|Default|GetDistance) (Variables|Default|GetSpeed)) (Spline|GetSplineLength _spline)))
  (Transformation|SetWorldLocation _train (Spline|GetLocationatDistanceAlongSpline _spline (Variables|Default|GetDistance) "World") false false)
  (Transformation|SetWorldRotation _train (Spline|GetRotationatDistanceAlongSpline _spline (Variables|Default|GetDistance) "World") false false))

(event EventBeginPlay
  ;[1 1 1] Play motor sound
  (Utilities|Time|SetTimerbyFunctionName 0 "MoveTrain" 0.01 true)
  (Audio|SpawnSoundAttached "/Game/ChristmasHoliday/Sounds/Train/Cue_TrainMotor.Cue_TrainMotor" (Variables|Default|GetTrain)))

(event EventTick
  (params (DeltaSeconds :type Float%20%28single-precision%29))
  ;[1 1 1] Play horn sound
  (Utilities|FlowControl|Delay (Math|Random|RandomFloatinRange 0.0 1e+01))
  (Audio|SpawnSoundAttached "/Game/ChristmasHoliday/Sounds/Train/Cue_TrainHorn01.Cue_TrainHorn01" (Variables|Default|GetTrain)))

(fn ConstructionScript
  (bind _spline (Variables|Default|GetSpline))
  (bind _spline_2 (Variables|Default|GetSpline))
  (bind _width (Variables|Default|GetWidth))
  (bind _returnvalue (Spline|GetLocationatDistanceAlongSpline _spline 0.0 "Local"))
  (Utilities|FlowControl|Sequence
    (:then_0
      (Spline|SetClosedLoop (Variables|Default|GetSpline) (Variables|Default|GetClose%20Looped%20Spline) true)
      ;[1 1 1] Loops spawning of spline mesh to cover spline distance
      (for _index (range 0 (- (Spline|GetNumberOfSplinePoints _spline_2) 1))
        (bind _returnvalue_2 (AddComponent|AddSplineMeshComponent false))
        ;[1 1 1] Set spline mesh and scale
        (Components|StaticMesh|SetStaticMesh _returnvalue_2 "/Game/ChristmasHoliday/Meshes/SM_TrainTrack01.SM_TrainTrack01")
        (Transformation|SetRelativeScale3D _returnvalue_2 (Math|Vector|MakeVector 1.0 _width _width))
        ;[1 1 1] Reorient mesh
        (SplineMesh|SetForwardAxis _returnvalue_2 "X" true)
        ;[1 1 1] Add the newly created mesh to the spline
        (Transformation|AttachComponentToComponent _returnvalue_2 (Variables|Default|GetSpline) "None" "KeepRelative" "KeepRelative" "KeepRelative" true)
        (SplineMesh|SetStartandEnd _returnvalue_2 (.Location (Spline|GetLocationandTangentatSplinePoint _spline_2 _index "Local")) (.Tangent (Spline|GetLocationandTangentatSplinePoint _spline_2 _index "Local")) (.Location (Spline|GetLocationandTangentatSplinePoint _spline_2 (+ _index 1) "Local")) (.Tangent (Spline|GetLocationandTangentatSplinePoint _spline_2 (+ _index 1) "Local")) true :!class /Script/Engine.SplineMeshComponent)))
    (:then_1
      ;[1 1 1] Spawn train
      (Variables|Default|SetLocation _returnvalue)
      (bind _returnvalue_3 (AddComponent|AddStaticMeshComponent true (Math|Transform|MakeTransform _returnvalue (Spline|GetRotationatDistanceAlongSpline _spline 0.0 "Local"))))
      (bind _output_get (Variables|Default|SetTrain _returnvalue_3))
      (Components|StaticMesh|SetStaticMesh _output_get "/Game/ChristmasHoliday/Meshes/SM_Train01.SM_Train01")
      (Transformation|AttachComponentToComponent _output_get (Variables|Default|GetSpline) "None" "KeepRelative" "KeepRelative" "KeepWorld" true))))