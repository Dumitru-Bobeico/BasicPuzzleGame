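; Decorative Christmas ornament string that is built along an editable, optionally looped spline in the construction script, with no active event logic.
; A wire spline mesh with adjustable width is stretched between each pair of spline points to form the cord.
; Ornament meshes are then added at a set spacing along the spline length, with configurable mesh, scale and rotation, each randomly given one of three materials.
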(event EventBeginPlay)

(event Collision|EventActorBeginOverlap
  (params (OtherActor :type Actor%20Object%20Reference)))

(event EventTick
  (params (DeltaSeconds :type Float%20%28single-precision%29)))

(fn ConstructionScript
  (bind _ornament_scale (Variables|Bulbs|GetOrnament%20Scale))
  (bind _spline (Variables|Default|GetSpline))
  (bind _ornamentspacing (Variables|Bulbs|GetOrnamentSpacing))
  (bind _width (Variables|Default|GetWidth))
  (bind _returnvalue (Math|Vector2D|MakeVector2D _width _width))
  (Utilities|FlowControl|Sequence
    (:then_0
      ;[1 1 1] Spawns cord
      (Spline|SetClosedLoop (Variables|Default|GetSpline) (Variables|Default|GetClose%20Looped%20Spline) true)
      ;;[1 1 1] Loops spawning of spline mesh to cover spline distance
      (for _index (range 0 (- (Spline|GetNumberOfSplinePoints _spline) 2))
        (bind _returnvalue_2 (AddComponent|AddSplineMeshComponent false))
        ;;[1 1 1] Set spline mesh and scale
        (Components|StaticMesh|SetStaticMesh _returnvalue_2 "/Game/ChristmasHoliday/Meshes/Wires/SM_SplineWire01.SM_SplineWire01")
        (SplineMesh|SetStartScale _returnvalue_2 _returnvalue true :!class /Script/Engine.SplineMeshComponent)
        (SplineMesh|SetEndScale _returnvalue_2 _returnvalue true :!class /Script/Engine.SplineMeshComponent)
        ;;[1 1 1] Reorient mesh
        (SplineMesh|SetForwardAxis _returnvalue_2 "Z" true)
        ;;[1 1 1] Add the newly created mesh to the spline
        (Transformation|AttachComponentToComponent _returnvalue_2 (Variables|Default|GetSpline) "None" "KeepRelative" "KeepRelative" "KeepRelative" true)
        (SplineMesh|SetStartandEnd _returnvalue_2 (.Location (Spline|GetLocationandTangentatSplinePoint _spline _index "Local")) (.Tangent (Spline|GetLocationandTangentatSplinePoint _spline _index "Local")) (.Location (Spline|GetLocationandTangentatSplinePoint _spline (+ _index 1) "Local")) (.Tangent (Spline|GetLocationandTangentatSplinePoint _spline (+ _index 1) "Local")) true :!class /Script/Engine.SplineMeshComponent)))
    (:then_1
      ;[1 1 1] Spawn Ornaments
      (for _index_2 (range 0 (.ReturnValue (Math|Float|Division(WholeandRemainder) (Spline|GetSplineLength _spline) _ornamentspacing)))
        (bind _returnvalue_3 (AddComponent|AddStaticMeshComponent true (Math|Transform|MakeTransform (Spline|GetLocationatDistanceAlongSpline _spline (* _index_2 _ornamentspacing) "Local") (Spline|GetRotationatDistanceAlongSpline _spline (* _index_2 _ornamentspacing) "Local"))))
        (Components|StaticMesh|SetStaticMesh _returnvalue_3 (Variables|Bulbs|GetOrnament%20Mesh))
        (Transformation|AddRelativeRotation _returnvalue_3 (Variables|Bulbs|GetOrnament%20Roation) false false)
        (Transformation|SetRelativeScale3D _returnvalue_3 (Math|Vector|MakeVector _ornament_scale _ornament_scale _ornament_scale))
        (switch int (Math|Random|RandomInteger 3)
          (:0
            (Rendering|Material|SetMaterial _returnvalue_3 0 "/Game/ChristmasHoliday/Materials/MI_Ornament01a.MI_Ornament01a"))
          (:1
            (Rendering|Material|SetMaterial _returnvalue_3 0 "/Game/ChristmasHoliday/Materials/MI_Ornament01b.MI_Ornament01b"))
          (:2
            (Rendering|Material|SetMaterial _returnvalue_3 0 "/Game/ChristmasHoliday/Materials/MI_Ornament01c.MI_Ornament01c")))
        (Transformation|AttachComponentToComponent _returnvalue_3 (Variables|Default|GetSpline) "None" "KeepRelative" "SnapToTarget" "KeepRelative" true)))))