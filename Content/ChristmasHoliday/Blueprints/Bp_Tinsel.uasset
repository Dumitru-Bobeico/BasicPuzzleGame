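; Christmas decoration actor that builds a tinsel garland along an editable spline, with optional light bulbs.
; The construction script stretches a tinsel spline mesh between each pair of spline points, with adjustable width and an option to set the spline as a closed loop.
; When bulbs are enabled, static mesh bulbs are placed at regular distances along the spline.
; Dynamic materials tint tinsel and bulbs with one shared colour and set bulb brightness.
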(event EventBeginPlay)

(event Collision|EventActorBeginOverlap
  (params (OtherActor :type Actor%20Object%20Reference)))

(event EventTick
  (params (DeltaSeconds :type Float%20%28single-precision%29)))

(fn ConstructionScript
  (bind _light_bulb_scale (Variables|Bulbs|GetLight%20Bulb%20Scale))
  (bind _spline (Variables|Default|GetSpline))
  (bind _light_bulb_spacing (Variables|Bulbs|GetLight%20Bulb%20Spacing))
  (bind _light_colour (Variables|Default|GetLight%20Colour))
  (bind _width (Variables|Default|GetWidth))
  (bind _returnvalue (Math|Vector2D|MakeVector2D _width _width))
  (Utilities|FlowControl|Sequence
    (:then_0
      ;[1 1 1] Spawns Tinsel
      (Spline|SetClosedLoop (Variables|Default|GetSpline) (Variables|Default|GetClose%20Looped%20Spline) true)
      ;;[1 1 1] Loops spawning of spline mesh to cover spline distance
      (for _index (range 0 (- (Spline|GetNumberOfSplinePoints _spline) 2))
        (bind _returnvalue_2 (AddComponent|AddSplineMeshComponent false))
        ;;[1 1 1] Set spline mesh and scale
        (Components|StaticMesh|SetStaticMesh _returnvalue_2 "/Game/ChristmasHoliday/Meshes/SM_Tinsel01a.SM_Tinsel01a")
        (bind _returnvalue_3 (Rendering|Material|CreateDynamicMaterialInstance _returnvalue_2 0 "/Game/ChristmasHoliday/Materials/MI_Tinsel01a.MI_Tinsel01a" :!class /Script/Engine.PrimitiveComponent))
        (Rendering|Material|SetVectorParameterValue _returnvalue_3 "Base Colour" _light_colour :!class /Script/Engine.MaterialInstanceDynamic)
        (SplineMesh|SetStartScale _returnvalue_2 _returnvalue true :!class /Script/Engine.SplineMeshComponent)
        (SplineMesh|SetEndScale _returnvalue_2 _returnvalue true :!class /Script/Engine.SplineMeshComponent)
        ;;[1 1 1] Reorient mesh
        (SplineMesh|SetForwardAxis _returnvalue_2 "X" true)
        ;;[1 1 1] Add the newly created mesh to the spline
        (Transformation|AttachComponentToComponent _returnvalue_2 (Variables|Default|GetSpline) "None" "KeepRelative" "KeepRelative" "KeepRelative" true)
        (SplineMesh|SetStartandEnd _returnvalue_2 (.Location (Spline|GetLocationandTangentatSplinePoint _spline _index "Local")) (.Tangent (Spline|GetLocationandTangentatSplinePoint _spline _index "Local")) (.Location (Spline|GetLocationandTangentatSplinePoint _spline (+ _index 1) "Local")) (.Tangent (Spline|GetLocationandTangentatSplinePoint _spline (+ _index 1) "Local")) true :!class /Script/Engine.SplineMeshComponent)))
    (:then_1
      ;[1 1 1] Spawn LightBulbs
      (if (Variables|Bulbs|GetUse%20Bulbs)
        (for _index_2 (range 0 (.ReturnValue (Math|Float|Division(WholeandRemainder) (Spline|GetSplineLength _spline) _light_bulb_spacing)))
          (bind _returnvalue_4 (AddComponent|AddStaticMeshComponent true (Math|Transform|MakeTransform (Spline|GetLocationatDistanceAlongSpline _spline (* _index_2 _light_bulb_spacing) "Local") (Spline|GetRotationatDistanceAlongSpline _spline (* _index_2 _light_bulb_spacing) "Local"))))
          (Components|StaticMesh|SetStaticMesh _returnvalue_4 (Variables|Bulbs|GetLight%20Bulb%20Mesh))
          (Transformation|AddRelativeRotation _returnvalue_4 (Variables|Bulbs|GetLight%20Relative%20Roation) false false)
          (Transformation|SetRelativeScale3D _returnvalue_4 (Math|Vector|MakeVector _light_bulb_scale _light_bulb_scale _light_bulb_scale))
          (bind _returnvalue_5 (Rendering|Material|CreateDynamicMaterialInstance _returnvalue_4 0 (Variables|Default|GetLight%20Material) :!class /Script/Engine.PrimitiveComponent))
          (Rendering|Material|SetVectorParameterValue _returnvalue_5 "Light Colour" _light_colour :!class /Script/Engine.MaterialInstanceDynamic)
          (Rendering|Material|SetScalarParameterValue _returnvalue_5 "Light Strength" (Variables|Default|GetLight%20Strength) :!class /Script/Engine.MaterialInstanceDynamic)
          (Transformation|AttachComponentToComponent _returnvalue_4 (Variables|Default|GetSpline) "None" "KeepRelative" "KeepRelative" "KeepRelative" true))))))