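; Shop prop dressing actor for the Christmas market, configured entirely in its construction script with no active event graph logic.
; A PropsOn switch shows or hides the Props hierarchy, and when on, three per-set toggles control each prop set's visibility with propagation to children.
; A ChairVariation option moves and rotates two of the chairs to fixed alternate placements.
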(event EventBeginPlay)

(event Collision|EventActorBeginOverlap
  (params (OtherActor :type Actor%20Object%20Reference)))

(event EventTick
  (params (DeltaSeconds :type Float%20%28single-precision%29)))

(fn ConstructionScript
  (bind _sm_chair2 (Variables|Default|GetSM_Chair2))
  (bind _propset_01 (Variables|Default|GetPropSet_01))
  (bind _propset_02 (Variables|Default|GetPropSet_02))
  (bind _sm_chair3 (Variables|Default|GetSM_Chair3))
  (bind _propset_03 (Variables|Default|GetPropSet_03))
  (bind _props (Variables|Default|GetProps))
  (if (Variables|Default|GetPropsOn?)
    (Rendering|SetVisibility _props true true)
    (if (Variables|Default|GetPropSet_01?)
      (Rendering|SetVisibility _propset_01 true true)
      (else
        (Rendering|SetVisibility _propset_01 false true)))
    (if (Variables|Default|GetPropSet_02?)
      (Rendering|SetVisibility _propset_02 true true)
      (else
        (Rendering|SetVisibility _propset_02 false true)))
    (if (Variables|Default|GetPropSet_03?)
      (Rendering|SetVisibility _propset_03 true true)
      (else
        (Rendering|SetVisibility _propset_03 false true)))
    (else
      (Rendering|SetVisibility _props false true)))
  (if (Variables|Default|GetChairVariation?)
    (Transformation|SetRelativeLocation _sm_chair2 "-96.127335,24.164501,0.000000" false false)
    (Transformation|SetRelativeRotation _sm_chair2 "0,-15.000000, 0" false false)
    (Transformation|SetRelativeLocation _sm_chair3 "82.712677,-5.620761,0.000549" false false)
    (Transformation|SetRelativeRotation _sm_chair3 "0.000000,172.000000,0.000000" false false)))