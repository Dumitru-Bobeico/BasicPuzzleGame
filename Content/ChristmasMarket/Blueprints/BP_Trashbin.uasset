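; BP_Trashbin is a Christmas market trash bin prop with an adjustable lid and optional garbage fill levels.
; The construction script sets the lid pivot's roll from LidRotation, clamped to 0–90 degrees, and toggles two extra garbage components by their flags.
; The fullest level raises the lid's minimum opening to 30 degrees.
; It has no runtime logic, as all event graph nodes are disabled stubs.
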(event EventBeginPlay)

(event Collision|EventActorBeginOverlap
  (params (OtherActor :type Actor%20Object%20Reference)))

(event EventTick
  (params (DeltaSeconds :type Float%20%28single-precision%29)))

(fn ConstructionScript
  (bind _moregarbage (Variables|Default|GetMoreGarbage))
  (bind _evenmoregarbage (Variables|Default|GetEvenMoreGarbage))
  (Transformation|SetRelativeRotation (Variables|Default|GetScene) (Math|Rotator|MakeRotator (Math|Float|Clamp(Float) (Variables|Default|GetLidRotation) 0.0 9e+01) 0.0 0.0) false false)
  (if (Variables|Default|GetMoreGarbage?)
    (Rendering|SetVisibility _moregarbage true true)
    (else
      (Rendering|SetVisibility _moregarbage false true)))
  (if (Variables|Default|GetEvenMoreGarbage?)
    (Rendering|SetVisibility _evenmoregarbage true true)
    (Transformation|SetRelativeRotation (Variables|Default|GetScene) (Math|Rotator|MakeRotator (Math|Float|Clamp(Float) (Variables|Default|GetLidRotation) 3e+01 9e+01) 0.0 0.0) false false)
    (else
      (Rendering|SetVisibility _evenmoregarbage false true))))