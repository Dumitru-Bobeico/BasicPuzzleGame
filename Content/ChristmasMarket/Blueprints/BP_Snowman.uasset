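; BP_Snowman is a configurable snowman prop for the Christmas Market that resolves its look in the construction script, with no active event logic.
; SnowmanVariation picks one of two snowman meshes, showing it and destroying the other component.
; For the first variant, HatOnOff and HatVariation select a Santa hat, a magician hat or none.
; The second variant always has both hat components destroyed.
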(event EventBeginPlay)

(event Collision|EventActorBeginOverlap
  (params (OtherActor :type Actor%20Object%20Reference)))

(event EventTick
  (params (DeltaSeconds :type Float%20%28single-precision%29)))

(fn ConstructionScript
  (bind _sm_snowman1 (Variables|Default|GetSM_Snowman1))
  (bind _sm_snowman (Variables|Default|GetSM_Snowman))
  (bind _sm_hat_magician_01 (Variables|Default|GetSM_Hat_Magician_01))
  (bind _sm_hat_santa_01 (Variables|Default|GetSM_Hat_Santa_01))
  (if (Variables|Default|GetSnowmanVariation?)
    (Rendering|SetVisibility _sm_snowman true false)
    (Components|DestroyComponent _sm_snowman1)
    (if (Variables|Default|GetHatOn/Off?)
      (if (Variables|Default|GetHatVariation)
        (Rendering|SetVisibility _sm_hat_santa_01 true false)
        (Components|DestroyComponent _sm_hat_magician_01)
        (else
          (Rendering|SetVisibility _sm_hat_magician_01 true false)
          (Components|DestroyComponent _sm_hat_santa_01)))
      (else
        (Components|DestroyComponent _sm_hat_santa_01 :!label _label)))
    (else
      (Rendering|SetVisibility _sm_snowman1 true false)
      (Components|DestroyComponent _sm_snowman)
      (goto _label))))