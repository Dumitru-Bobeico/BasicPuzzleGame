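; BP_Light_01 is a configurable point light actor for the Christmas Market scene.
; Its construction script applies exposed intensity, radius, color and shadow settings to the PointLight component, scaling intensity by a multiplier and zeroing source radius.
; When LightOnOff is false, the script destroys the light component instead; the event graph holds no active logic.
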(event EventBeginPlay)

(event Collision|EventActorBeginOverlap
  (params (OtherActor :type Actor%20Object%20Reference)))

(event EventTick
  (params (DeltaSeconds :type Float%20%28single-precision%29)))

(fn ConstructionScript
  (bind _pointlight (Variables|Default|GetPointLight))
  (if (Variables|Default|GetLightOn/Off)
    (Rendering|Components|Light|SetIntensity _pointlight (* (Variables|Default|GetIntensity) 1e+02))
    (Rendering|Lighting|SetAttenuationRadius _pointlight (Variables|Default|GetRadius))
    (Class|PointLightComponent|SetSourceRadius _pointlight 0.0)
    (Rendering|Components|Light|SetLightColor _pointlight (Variables|Default|GetColor) true)
    (Rendering|Components|Light|SetCastShadows _pointlight (Variables|Default|GetCastShadows?))
    (else
      (Components|DestroyComponent (Variables|Default|GetPointLight)))))