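; Christmas market stand actor with optional snow globe effects and lighting, configured per placed instance in the construction script.
; The SnowGlobeOnOff flag shows or hides three Niagara components.
; LightsOnOff applies intensity (scaled by 100), radius, color and shadow settings to the point light, or destroys it along with two rect lights when off.
; The event graph holds no active logic.
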(event EventBeginPlay)

(event Collision|EventActorBeginOverlap
  (params (OtherActor :type Actor%20Object%20Reference)))

(event EventTick
  (params (DeltaSeconds :type Float%20%28single-precision%29)))

(fn ConstructionScript
  (bind _niagara1 (Variables|Default|GetNiagara1))
  (bind _niagara2 (Variables|Default|GetNiagara2))
  (bind _niagara (Variables|Default|GetNiagara))
  (bind _pointlight (Variables|Default|GetPointLight))
  (if (Variables|Default|GetSnowGlobe%20On/Off)
    (Rendering|SetVisibility _niagara true false)
    (Rendering|SetVisibility _niagara1 true false)
    (Rendering|SetVisibility _niagara2 true false)
    (else
      (Rendering|SetVisibility _niagara false false)
      (Rendering|SetVisibility _niagara1 false false)
      (Rendering|SetVisibility _niagara2 false false)))
  (if (Variables|Default|GetLightsOn/Off?)
    (Rendering|Components|Light|SetIntensity _pointlight (* (Variables|Default|GetIntensity) 1e+02))
    (Rendering|Lighting|SetAttenuationRadius _pointlight (Variables|Default|GetRadius))
    (Rendering|Components|Light|SetLightColor _pointlight (Variables|Default|GetColor) true)
    (Rendering|Components|Light|SetCastShadows _pointlight (Variables|Default|GetCastShadows?))
    (else
      (Components|DestroyComponent _pointlight))))